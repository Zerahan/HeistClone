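; Endlessly scrolling road actor that fakes forward movement by sliding instanced scenery backward.
; The construction script builds mirrored road and sidewalk instances along X, with grass tiles on both sides sized by RoadLength and LandscapeWidth.
; Tick pans PanningComponent with a modulo wrap, optionally swaying it sideways on a cosine between YBounds.
; It passes the same motion to InfiniteMovingForest to keep it in step.
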(event EventTick
  (params (DeltaSeconds :type Float%20%28single-precision%29))
  (bind _panspeed (Variables|Default|GetPanSpeed))
  (bind _ybounds (Variables|Default|GetYBounds))
  (bind (_x _y) (Math|Vector2D|BreakVector2D _ybounds))
  (bind _returnvalue (* DeltaSeconds _panspeed))
  (Variables|Default|SetCurrentXPosition (Math|Float|%(Float) (+ (* _returnvalue -1.0) (Variables|Default|GetCurrentXPosition)) (* (.X (Math|Vector|BreakVector (Variables|/Script/Engine.SceneComponent|GetRelativeScale3D (Variables|Default|GetPanningComponent)))) 1e+03)))
  (if (> (Math|Vector2D|Vector2DLength (Variables|Default|GetYBounds)) 0.0)
    (Variables|Default|SetCurrentYPosition (|(((0.500000*((cos((((4*x)*pi)/(2*c))))+1))*(b-a))+a) (Utilities|Time|GetGameTimeinSeconds) (Math|Trig|GetPI) (Variables|Default|GetYSpeed) _y _x)))
  (Default|UpdatePosition (Variables|Default|GetInfiniteMovingForest) _returnvalue (Variables|Default|GetCurrentYPosition))
  (Transformation|SetRelativeLocation (Variables|Default|GetPanningComponent) (Math|Vector|MakeVector (Variables|Default|GetCurrentXPosition) (Variables|Default|GetCurrentYPosition) 0.0) false false))

(fn ConstructionScript
  (bind _panningcomponent (Variables|Default|GetPanningComponent))
  (bind _relativescale3d (Variables|/Script/Engine.SceneComponent|GetRelativeScale3D _panningcomponent))
  (bind _x (Math|Vector|BreakVector _relativescale3d))
  (bind _returnvalue (Math|Vector|MakeVector 1.0 _x 1.0))
  (for _index (range 0 (- (Variables|Default|GetRoadLength) 1))
    (Components|InstancedStaticMesh|AddInstance (Variables|Default|GetSidewalk) (Math|Transform|MakeTransform (Math|Vector|MakeVector (Math|Conversions|ToFloat(Integer) (* _index 500)) -5e+02 0.0)))
    (Components|InstancedStaticMesh|AddInstance (Variables|Default|GetRoad) (Math|Transform|MakeTransform (Math|Vector|MakeVector (Math|Conversions|ToFloat(Integer) (* _index 500)) -5e+02 0.0) "0,90.000000, 0"))
    (Components|InstancedStaticMesh|AddInstance (Variables|Default|GetSidewalk) (Math|Transform|MakeTransform (Math|Vector|MakeVector (Math|Conversions|ToFloat(Integer) (+ (* _index 500) 500)) 5e+02 0.0) "0,180.000000, 0"))
    (Components|InstancedStaticMesh|AddInstance (Variables|Default|GetRoad) (Math|Transform|MakeTransform (Math|Vector|MakeVector (Math|Conversions|ToFloat(Integer) (+ (* _index 500) 500)) 5e+02 0.0) "0,270.000000, 0"))
    (for _index_2 (range 0 (- (Variables|Default|GetLandscapeWidth) 1))
      (Components|InstancedStaticMesh|AddInstance (Variables|Default|GetGrass) (Math|Transform|MakeTransform (Math|Vector|MakeVector (Math|Conversions|ToFloat(Integer) (* _index 500)) (+ (* (* (* _index_2 500) _x) -1.0) -1e+03) 0.0) "0,0.000000, 0" _returnvalue))
      (Components|InstancedStaticMesh|AddInstance (Variables|Default|GetGrass) (Math|Transform|MakeTransform (Math|Vector|MakeVector (Math|Conversions|ToFloat(Integer) (* _index 500)) (+ (* (* _index_2 500) _x) 3e+03) 0.0) "0,0.000000, 0" _returnvalue)))))