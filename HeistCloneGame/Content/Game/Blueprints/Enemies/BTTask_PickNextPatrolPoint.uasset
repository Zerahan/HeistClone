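; Behavior tree task that picks the next patrol point for an EnemyGuard and stores it in the blackboard.
; It asks the guard for its next point, then writes that point's location and facing direction to blackboard keys.
; It also writes whether to wait there from the PatrolPoint's WaitHere flag, defaulting to waiting when the reference is not a PatrolPoint, then finishes successfully.
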(event `self.ReceiveExecuteAI`
  (params (OwnerController :type "AIController Object Reference") (ControlledPawn :type "Pawn Object Reference"))
  (bind _asenemy_guard (cast `/Game/Game/Blueprints/Enemies/EnemyGuard` ControlledPawn))
  (bind (_nextpatrolpoint _patrolpointref _direction) (`/Game/Game/Blueprints/Enemies/EnemyGuard.GetNextPatrolPoint` _asenemy_guard))
  (`BTFunctionLibrary.SetBlackboardValueAsVector` (`self.PatrolPointLocationBBKey`) (`Actor.K2_GetActorLocation` _patrolpointref))
  (`BTFunctionLibrary.SetBlackboardValueAsVector` (`self.PatrolPointFacingDirectionBBKey`) _direction)
  (bind _aspatrol_point (cast `/Game/Game/Blueprints/Enemies/PatrolPoint` _patrolpointref)
    (:`then`
      (`BTFunctionLibrary.SetBlackboardValueAsBool` (`self.WaitsAtPatrolPoint`) (`/Game/Game/Blueprints/Enemies/PatrolPoint.WaitHere` _aspatrol_point)))
    (:`CastFailed`
      (`BTFunctionLibrary.SetBlackboardValueAsBool` (`self.WaitsAtPatrolPoint`) true)))
  (`self.FinishExecute` true))