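; A damageable dev cube, filed under Enemies, that displays its health as color and broadcasts its death.
; The construction script creates a dynamic material instance on the cube.
; Damage lowers clamped health and refreshes the Color parameter, which shifts from green to red and turns black at zero.
; The first drop to zero clears IsAlive and fires OnKilled, while IsDead reports whether health is depleted.
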(event `self.ReceiveBeginPlay`
  (`self.UpdateGraphics`))

(event `self.ReceiveAnyDamage`
  (params (Damage :type "Float (single-precision)") (DamageType :type "DamageType Object Reference") (InstigatedBy :type "Controller Object Reference") (DamageCauser :type "Actor Object Reference"))
  (set `self.CurrentHealth` (`KismetMathLibrary.FClamp` (- (`self.CurrentHealth`) Damage) 0.0 (`self.MaximumHealth`)))
  (`self.UpdateGraphics`)
  (if (`self.IsAlive`)
    (if (<= (`self.CurrentHealth`) 0.0)
      (set `self.IsAlive` false)
      (`self.OnKilled`))))

(fn `IsDead`
  (returns (IsDead :type Boolean))
  (return (<= (`self.CurrentHealth`) 0.0)))

(fn `UpdateGraphics`
  (`MaterialInstanceDynamic.SetVectorParameterValue` (`self.DynamicMatInstance`) "Color" (select `bool` (> (`self.CurrentHealth`) 0.0) :`true` (`KismetMathLibrary.MakeColor` (- 1.0 (/ (`self.CurrentHealth`) (`self.MaximumHealth`))) (/ (`self.CurrentHealth`) (`self.MaximumHealth`))))))

(fn `UserConstructionScript`
  (`/Engine/EditorBlueprintResources/StandardMacros.IsValid` (`self.DynamicMatInstance`)
    (:`Is Not Valid`
      (bind _returnvalue (`PrimitiveComponent.CreateDynamicMaterialInstance` (`self.Cube`) 0 (`PrimitiveComponent.GetMaterial` (`self.Cube`) 0) "None"))
      (bind _output_get (set `self.DynamicMatInstance` _returnvalue))
      (`PrimitiveComponent.SetMaterial` (`self.Cube`) 0 _output_get))))