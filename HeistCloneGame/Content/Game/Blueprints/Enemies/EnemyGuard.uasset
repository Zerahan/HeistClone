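; Heist-game AI character serving as either a police guard or a civilian, with TriggersPager choosing its random mesh, color, light cone and which death the GameState records.
; It runs a behavior tree, with helpers supplying unblocked patrol points.
; Sight perception feeds DetectionHandler and its alert widget; detection or the world alarm sets IsAlerted.
; Any damage kills it regardless of remaining health, clearing detections and dropping a LootBag.
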(event `WorldAlarm`
  (set `self.IsAlerted` true :!label _label))

(event `self.ReceiveBeginPlay`
  (`|ExecutionSequence`
    (:`then_0`
      (if (> (`KismetArrayLibrary.Array_Length` (`self.PatrolPoints`)) 0)
        (if (`self.UseRandomStart`)
          (bind (_patrolpoint _chosenindex) (`self.GetRandomPatrolPoint` false))
          (set `self.NextPatrolPoint` (mod (+ _chosenindex 1) (`KismetArrayLibrary.Array_Length` (`self.PatrolPoints`))))
          (`self.K2_SetActorLocation` (`self.K2_GetActorLocation` _patrolpoint))
          (else
            (`self.K2_SetActorLocation` (`self.K2_GetActorLocation` (`|GetArrayItem` (`self.PatrolPoints`))))))))
    (:`then_1`
      (bind _returnvalue (`|CreateWidget` "/Game/Game/UI/EnemyAlertWidget.EnemyAlertWidget_C" null self (`self.DetectionHandler`)))
      (`/Game/Game/UI/EnemyAlertWidget.Initialize` _returnvalue)
      (`WidgetComponent.SetWidget` (`self.DetectionWidget`) _returnvalue)
      (`AIController.RunBehaviorTree` (`AIBlueprintHelperLibrary.GetAIController` self) "/Game/Game/Blueprints/Enemies/Behavior/GuardBehavior.GuardBehavior")
      (add `/Game/Game/Blueprints/Enemies/Behavior/DetectionHandler.OnAlert` (`self.DetectionHandler`) (delegate `Alerted`))
      (bind _asheist_game_clone_game_state (cast `/Game/Game/Blueprints/HeistGameCloneGameState` (`GameplayStatics.GetGameState`)))
      (add `/Game/Game/Blueprints/HeistGameCloneGameState.UpdateAlarmState` _asheist_game_clone_game_state (delegate `WorldAlarm`)))
    (:`then_2`
      (if (not (`self.TriggersPager`))
        (set `CharacterMovementComponent.MaxWalkSpeed` 100.0 (`self.CharacterMovement`))
        (set `/Game/Game/Blueprints/Enemies/Behavior/DetectionHandler.MaxDetectionTime` 12.0 (`self.DetectionHandler`))))))

(event `Alerted`
  (goto _label))

(event `self.AIPerception.OnTargetPerceptionUpdated`
  (params (Actor :type "Actor Object Reference") (Stimulus :type "AIStimulus Structure"))
  (bind (_age _expirationage _strength _stimuluslocation _receiverlocation _tag _bsuccessfullysensed) (break `AIStimulus` Stimulus))
  (bind _detectionhandler (`self.DetectionHandler`))
  (`/Engine/EditorBlueprintResources/StandardMacros.IsValid` _detectionhandler
    (:`Is Valid`
      (if (not (and (not (`self.TriggersPager`)) (`KismetMathLibrary.ClassIsChildOf` (`GameplayStatics.GetObjectClass` Actor) "/Game/Game/Props/LootBox.LootBox_C")))
        (if (`/Game/Game/Blueprints/Enemies/Behavior/DetectionHandler.CanDetectActorClass` (`self.DetectionHandler`) Actor)
          (if (`/Game/Game/Blueprints/Enemies/Behavior/DetectionHandler.GetCanDetect` _detectionhandler)
            (`/Engine/EditorBlueprintResources/StandardMacros.IsValid` Actor
              (:`Is Valid`
                (`/Game/Game/Blueprints/Enemies/Behavior/DetectionHandler.SetDetected` (`self.DetectionHandler`) _bsuccessfullysensed Actor)
                (bind _asheist_game_clone_character (cast `/Game/Game/Blueprints/HeistGameCloneCharacter` Actor))
                (if _bsuccessfullysensed
                  (`/Game/Game/Blueprints/HeistGameCloneCharacter.RegisterDetection` _asheist_game_clone_character self)
                  (else
                    (`/Game/Game/Blueprints/HeistGameCloneCharacter.UnregisterDetection` _asheist_game_clone_character self))))
              (:`Is Not Valid`
                (`/Game/Game/Blueprints/Enemies/Behavior/DetectionHandler.SetDetected` (`self.DetectionHandler`) false Actor)))))))))

(event `self.ReceiveAnyDamage`
  (params (Damage :type "Float (single-precision)") (DamageType :type "DamageType Object Reference") (InstigatedBy :type "Controller Object Reference") (DamageCauser :type "Actor Object Reference"))
  (set `self.CurrentHealth` (`KismetMathLibrary.FClamp` (- (`self.CurrentHealth`) Damage) 0.0 (`self.MaxHealth`)))
  (if (`self.IsAlive`)
    (`self.OnKilled`)
    (set `self.IsAlive` false)
    (for _array_element (`AIPerceptionComponent.GetKnownPerceivedActors` (`self.AIPerception`) null)
      (bind _asheist_game_clone_character (cast `/Game/Game/Blueprints/HeistGameCloneCharacter` _array_element))
      (`/Game/Game/Blueprints/HeistGameCloneCharacter.UnregisterDetection` _asheist_game_clone_character self))
    (`AIPerceptionComponent.SetSenseEnabled` (`self.AIPerception`) "/Script/AIModule.AISense_Sight" false)
    (`|SpawnActorFromClass` "/Game/Game/Props/LootBag.LootBag_C" (`self.GetTransform`) "Undefined" "OverrideRootScale" null "NewEnumerator0" null)
    (`self.K2_DestroyActor`)))

(event `self.ReceiveDestroyed`
  (`parent.ReceiveDestroyed`)
  (`self.OnKilled`)
  (if (`self.TriggersPager`)
    (bind _asheist_game_clone_game_state (cast `/Game/Game/Blueprints/HeistGameCloneGameState` (`GameplayStatics.GetGameState`)))
    (`/Game/Game/Blueprints/HeistGameCloneGameState.RegisterGuardDeath` _asheist_game_clone_game_state)
    (else
      (bind _asheist_game_clone_game_state_2 (cast `/Game/Game/Blueprints/HeistGameCloneGameState` (`GameplayStatics.GetGameState`)))
      (`/Game/Game/Blueprints/HeistGameCloneGameState.RegisterCivilianDeath` _asheist_game_clone_game_state_2))))

(fn `GetNextPatrolPoint`
  (returns (NextPatrolPoint :type Integer) (PatrolPointRef :type "Actor Object Reference") (Direction :type "Vector Structure"))
  (bind _output (`|GetArrayItem` (`self.PatrolPoints`) (`self.NextPatrolPoint`)))
  (if (!= (`KismetArrayLibrary.Array_Length` (`self.PatrolPoints`)) 0)
    (set `self.NextPatrolPoint` (mod (+ (`self.NextPatrolPoint`) 1) (`KismetArrayLibrary.Array_Length` (`self.PatrolPoints`))) :!label _label)
    (bind _isblocked (`/Game/Game/Blueprints/Enemies/PatrolPoint.IsBlocked` _output))
    (if _isblocked
      (goto _label)
      (else
        (return (`self.NextPatrolPoint`) _output (`self.GetActorForwardVector` _output))))
    (else
      (return 0 self (`self.GetActorForwardVector`)))))

(fn `GetRandomPatrolPoint`
  (params (IncludeInvalidStarts :type Boolean))
  (returns (PatrolPoint :type "/Game/Game/Blueprints/Enemies/PatrolPoint Object Reference") (ChosenIndex :type Integer))
  (locals (LocalPatrolPoints :type "Array of /Game/Game/Blueprints/Enemies/PatrolPoint Object Reference") (LocalChosenIndex :type Integer :default 0))
  (bind _patrolpoints (`self.PatrolPoints`))
  (bind _output (`|GetArrayItem` (`local.LocalPatrolPoints`) (`KismetMathLibrary.RandomIntegerInRange` 0 (- (`KismetArrayLibrary.Array_Length` (`self.PatrolPoints`)) 1))))
  (if IncludeInvalidStarts
    (set `local.LocalPatrolPoints` _patrolpoints)
    (else
      (for _array_element (`self.PatrolPoints`)
        (bind _isblocked (`/Game/Game/Blueprints/Enemies/PatrolPoint.IsBlocked` _array_element))
        (if (not _isblocked)
          (`KismetArrayLibrary.Array_Add` (`local.LocalPatrolPoints`) _array_element)))))
  (return _output (`KismetArrayLibrary.Array_Find` _patrolpoints _output)))

(fn `IsDead`
  (returns (IsDead :type Boolean))
  (return (not (`self.IsAlive`))))

(fn `UserConstructionScript`
  (bind _staticmesh (`self.StaticMesh`))
  (bind _returnvalue (`PrimitiveComponent.CreateDynamicMaterialInstance` _staticmesh 0 (`PrimitiveComponent.GetMaterial` _staticmesh 0) "None"))
  (`MaterialInstanceDynamic.SetVectorParameterValue` _returnvalue "Color" (select `bool` (`self.TriggersPager`) :`false` (struct :`R` 0.5 :`G` 1.0 :`B` 1.0 :`A` 1.0) :`true` (struct :`R` 1.0 :`G` 0.5 :`B` 0.5 :`A` 1.0) :!type "LinearColor Structure"))
  (`PrimitiveComponent.SetMaterial` (`self.StaticMesh`) 0 _returnvalue)
  (`SceneComponent.SetVisibility` (`self.LightCone`) (`self.TriggersPager`) false)
  (`SkinnedMeshComponent.SetSkinnedAssetAndUpdate` (`self.Mesh`) (select `bool` (`self.TriggersPager`) :`false` (select `int` (`KismetMathLibrary.RandomInteger` 7) :`0` "/Game/Packages/PolygonCity/Meshes/Characters/SK_Character_BusinessMan_Shirt.SK_Character_BusinessMan_Shirt" :`1` "/Game/Packages/PolygonCity/Meshes/Characters/SK_Character_BusinessMan_Suit.SK_Character_BusinessMan_Suit" :`2` "/Game/Packages/PolygonCity/Meshes/Characters/SK_Character_BusinessWoman.SK_Character_BusinessWoman" :`3` "/Game/Packages/PolygonCity/Meshes/Characters/SK_Character_Female_Coat.SK_Character_Female_Coat" :`4` "/Game/Packages/PolygonCity/Meshes/Characters/SK_Character_Female_Jacket.SK_Character_Female_Jacket" :`5` "/Game/Packages/PolygonCity/Meshes/Characters/SK_Character_Male_Hoodie.SK_Character_Male_Hoodie" :`6` "/Game/Packages/PolygonCity/Meshes/Characters/SK_Character_Male_Jacket.SK_Character_Male_Jacket" :!type "SkeletalMesh Object Reference") :`true` (select `int` (`KismetMathLibrary.RandomInteger` 2) :`0` "/Game/Packages/PolygonCity/Meshes/Characters/SK_Character_Male_Police.SK_Character_Male_Police" :`1` "/Game/Packages/PolygonCity/Meshes/Characters/SK_Character_Female_Police.SK_Character_Female_Police" :!type "SkeletalMesh Object Reference")) true))