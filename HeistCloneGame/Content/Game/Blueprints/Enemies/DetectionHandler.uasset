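; Enemy detection component for a heist game that tracks seen actors and moves its owner through idle, detecting, alerted, alarm-calling and confused states.
; Paired heat-up and cooldown timers carry partial progress when sight changes, with Tick clearing destroyed actors.
; Full detection alerts, then delayed calls trigger the GameState alarm unless the owner or optional operator is dead.
; Dispatchers announce changes, while getters expose alert progress and timed confusion.
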(event `self.ReceiveBeginPlay`
  (bind _operator (`self.Operator`))
  (bind _asheist_game_clone_game_state (cast `/Game/Game/Blueprints/HeistGameCloneGameState` (`GameplayStatics.GetGameState`)))
  (add `/Game/Game/Blueprints/HeistGameCloneGameState.UpdateAlarmState` _asheist_game_clone_game_state (`|CreateDelegate` :!event `WorldAlarm`))
  (`/Engine/EditorBlueprintResources/StandardMacros.IsValid` _operator
    (:`Is Valid`
      (add `Actor.OnDestroyed` _operator (delegate `OperatorKilled`)))))

(event `OperatorKilled`
  (params (DestroyedActor :type "Actor Object Reference"))
  (set `self.IsOperatorDead` true)
  (`self.OnOperatorKilled`))

(event `self.ReceiveTick`
  (params (DeltaSeconds :type "Float (single-precision)"))
  ;[1 1 1] For seen actors that are destroyed - like loot bags that are picked up
  (for _array_element (`self.SeenActors`)
    (`/Engine/EditorBlueprintResources/StandardMacros.IsValid` _array_element
      (:`Is Not Valid`
        (`self.SetDetected` false _array_element)))))

(event `Reset`
  (set `self.IsHeatingUp` false)
  (`KismetSystemLibrary.K2_ClearAndInvalidateTimerHandle` (`self.AlarmTimerHandle`))
  (`KismetSystemLibrary.K2_ClearAndInvalidateTimerHandle` (`self.CooldownTimerHandle`))
  (set `self.IsIdle` true)
  (set `self.TimerOffset` 0.0))

(event `SetDetected`
  (params (IsHeatingUp :type Boolean) (SeenActor :type "Actor Object Reference"))
  (bind _maxdetectiontime (`self.MaxDetectionTime`))
  (bind _returnvalue (`KismetSystemLibrary.K2_GetTimerRemainingTimeHandle` (`self.CooldownTimerHandle`)))
  (bind _returnvalue_2 (+ (`KismetSystemLibrary.K2_GetTimerElapsedTimeHandle` (`self.AlarmTimerHandle`)) (`self.TimerOffset`)))
  (bind _returnvalue_3 (select `bool` (`KismetSystemLibrary.K2_IsValidTimerHandle` (`self.CooldownTimerHandle`)) :`false` _maxdetectiontime :`true` (- _maxdetectiontime _returnvalue)))
  (if (and (not (`self.IsAlerted`)) (not (`self.IsCallingAlarm`)) (`self.GetCanDetect`))
    (`self.ModSeenActors` IsHeatingUp SeenActor)
    (if (!= IsHeatingUp (`self.IsHeatingUp`))
      (if (`self.IsIdle`)
        (`self.OnWake`))
      (set `self.IsIdle` false)
      (bind _output_get (set `self.IsHeatingUp` IsHeatingUp))
      (if _output_get
        (set `self.TimerOffset` _returnvalue)
        (set `self.TimeDuration` _returnvalue_3)
        (bind _returnvalue_4 (`KismetSystemLibrary.K2_SetTimerDelegate` (`|CreateDelegate` :!event `OnHeated`) _returnvalue_3))
        (set `self.AlarmTimerHandle` _returnvalue_4)
        (`KismetSystemLibrary.K2_ClearAndInvalidateTimerHandle` (`self.CooldownTimerHandle`))
        (elif (== (`KismetArrayLibrary.Array_Length` (`self.SeenActors`)) 0)
          (if (`KismetSystemLibrary.K2_IsValidTimerHandle` (`self.AlarmTimerHandle`))
            (set `self.TimeDuration` _returnvalue_2)
            (bind _returnvalue_5 (`KismetSystemLibrary.K2_SetTimerDelegate` (`|CreateDelegate` :!event `OnCooled`) _returnvalue_2))
            (set `self.CooldownTimerHandle` _returnvalue_5)
            (`KismetSystemLibrary.K2_ClearAndInvalidateTimerHandle` (`self.AlarmTimerHandle`))
            (set `self.TimerOffset` 0.0))
          (else
            (set `self.IsHeatingUp` true)))))))

(event `OnCooled`
  (set `self.IsIdle` true)
  (set `self.TimerOffset` 0.0)
  (`KismetSystemLibrary.K2_ClearAndInvalidateTimerHandle` (`self.CooldownTimerHandle`))
  (`self.OnIdle`))

(event `WorldAlarm`
  (`self.OnWake`)
  (set `self.IsAlerted` true :!label _label)
  (`self.OnAlert`))

(event `OnHeated`
  (`KismetSystemLibrary.K2_ClearAndInvalidateTimerHandle` (`self.AlarmTimerHandle`))
  (`KismetSystemLibrary.K2_SetTimerDelegate` (delegate `CallAlarm`) 4.0)
  (goto _label))

(event `CallAlarm`
  (if (`self.GetCanCallAlarm`)
    (`KismetSystemLibrary.K2_SetTimerDelegate` (delegate `FinishAlarm`) 2.0)
    (set `self.IsCallingAlarm` true)
    (`self.OnAlarm`)))

(event `FinishAlarm`
  (set `self.IsIdle` true)
  (if (`self.GetCanCallAlarm`)
    (set `self.IsCallingAlarm` false)
    (`self.DoAlarm`)
    (bind _asheist_game_clone_game_state (cast `/Game/Game/Blueprints/HeistGameCloneGameState` (`GameplayStatics.GetGameState`)))
    (`/Game/Game/Blueprints/HeistGameCloneGameState.SetOffAlarm` _asheist_game_clone_game_state)))

(event `Confuse`
  (if (`self.CanConfuse`)
    (`self.SetIsConfused` true)
    (`KismetSystemLibrary.K2_ClearAndInvalidateTimerHandle` (`self.ConfuseTimerHandle`))
    (bind _returnvalue (`KismetSystemLibrary.K2_SetTimerDelegate` (delegate `DoEndConfusion`) (`self.ConfuseDuration`)))
    (set `self.ConfuseTimerHandle` _returnvalue)
    (`self.OnConfusionUpdate`)))

(event `DoEndConfusion`
  (`KismetSystemLibrary.K2_ClearAndInvalidateTimerHandle` (`self.ConfuseTimerHandle`))
  (`self.SetIsConfused` false)
  (`self.OnConfusionUpdate`))

(fn `CanConfuse`
  (returns (CanConfuse :type Boolean))
  (return (and (not (`self.IsAlerted`)) (`self.IsConfusionEnding`))))

(fn `CanDetectActorClass`
  (params (Actor :type "Actor Object Reference"))
  (returns (CanDetect :type Boolean))
  (bind _returnvalue (`GameplayStatics.GetObjectClass` Actor))
  (`/Engine/EditorBlueprintResources/StandardMacros.IsValid` Actor
    (:`Is Valid`
      (bind _isdead (message `/Game/Game/Blueprints/HealthInterface.IsDead` Actor))
      (return (not (or (`KismetMathLibrary.ClassIsChildOf` _returnvalue "/Game/Game/Blueprints/Enemies/EnemyGuard.EnemyGuard_C") (and (`KismetMathLibrary.ClassIsChildOf` _returnvalue "/Game/Game/Blueprints/Enemies/EnemyCamera.EnemyCamera_C") (not _isdead))))))
    (:`Is Not Valid`
      (return false))))

(fn `GetAlertDuration`
  (returns (AlertDuration :type "Float (double-precision)"))
  (return (`self.MaxDetectionTime`)))

(fn `GetAlertLevel`
  (returns (AlertLevel :type "Float (double-precision)"))
  (return (+ (select `bool` (`self.IsHeatingUp`) :`false` (`KismetSystemLibrary.K2_GetTimerRemainingTimeHandle` (`self.CooldownTimerHandle`)) :`true` (`KismetSystemLibrary.K2_GetTimerElapsedTimeHandle` (`self.AlarmTimerHandle`))) (`self.TimerOffset`))))

(fn `GetAlertPercent`
  (returns (AlertPercent :type "Float (double-precision)"))
  (return (select `bool` (`self.IsAlerted`) :`false` (/ (`self.GetAlertLevel`) (`self.MaxDetectionTime`)) :`true` 1.0)))

(fn `GetCanCallAlarm`
  (returns (CanCallAlarm :type Boolean))
  (bind _isdead (message `/Game/Game/Blueprints/HealthInterface.IsDead` (`self.GetOwner`)))
  (`/Engine/EditorBlueprintResources/StandardMacros.IsValid` (`self.Operator`)
    (:`Is Valid`
      (bind _isdead_2 (message `/Game/Game/Blueprints/HealthInterface.IsDead` (`self.Operator`)))
      (bind _returnvalue (not _isdead))
      (return (and (not _isdead_2) _returnvalue)))
    (:`Is Not Valid`
      (return (and _returnvalue (not (`self.IsOperatorDead`)))))))

(fn `GetCanDetect`
  (returns (CanDetect :type Boolean))
  (bind _isdead (message `/Game/Game/Blueprints/HealthInterface.IsDead` (`self.GetOwner`)))
  (if _isdead
    (return false)
    (else
      (`/Engine/EditorBlueprintResources/StandardMacros.IsValid` (`self.Operator`)
        (:`Is Valid`
          (bind _isdead_2 (message `/Game/Game/Blueprints/HealthInterface.IsDead` (`self.Operator`)))
          (return (not _isdead_2)))
        (:`Is Not Valid`
          (return (not (`self.IsOperatorDead`))))))))

(fn `GetConfusionRemaining`
  (returns (Remaining :type "Float (double-precision)"))
  (if (`KismetSystemLibrary.K2_IsValidTimerHandle` (`self.ConfuseTimerHandle`))
    (return (`KismetSystemLibrary.K2_GetTimerRemainingTimeHandle` (`self.ConfuseTimerHandle`)))
    (else
      (return -1.0))))

(fn `GetDetectionState`
  (returns (DetectionState :type "/Game/Game/Blueprints/EDetectionState Enum"))
  (return (select `bool` (`self.IsCallingAlarm`) :`false` (select `bool` (`self.IsConfused`) :`false` (select `bool` (`self.IsAlerted`) :`false` (select `bool` (`self.IsIdle`) :`false` "NewEnumerator1" :`true` "NewEnumerator0" :!type "/Game/Game/Blueprints/EDetectionState Enum") :`true` "NewEnumerator2") :`true` "NewEnumerator4") :`true` "NewEnumerator3")))

(fn `GetEndTime`
  (returns (IsIncreasingPercent :type Boolean) (AlertEndTime :type "Float (double-precision)") (AlertDuration :type "Float (double-precision)"))
  (bind _isheatingup (`self.IsHeatingUp`))
  (return _isheatingup (+ (select `bool` _isheatingup :`false` (`KismetSystemLibrary.K2_GetTimerRemainingTimeHandle` (`self.CooldownTimerHandle`)) :`true` (`KismetSystemLibrary.K2_GetTimerRemainingTimeHandle` (`self.AlarmTimerHandle`))) (`KismetSystemLibrary.GetGameTimeInSeconds`)) (`self.MaxDetectionTime`)))

(fn `GetIsConfused`
  (returns (IsConfused :type Boolean))
  (return (`self.IsConfused`)))

(fn `GetOperator`
  (returns (Operator :type "Actor Object Reference"))
  (return (`self.Operator`)))

(fn `IsConfusionEnding`
  (returns (IsEnding :type Boolean))
  (if (`KismetSystemLibrary.K2_IsValidTimerHandle` (`self.ConfuseTimerHandle`))
    (return (< (`KismetSystemLibrary.K2_GetTimerRemainingTimeHandle` (`self.ConfuseTimerHandle`)) 5.0))
    (else
      (return true))))

(fn `ModSeenActors`
  (params (IsCurrentlySeen :type Boolean) (SeenActor :type "Actor Object Reference"))
  (if IsCurrentlySeen
    (`KismetArrayLibrary.Array_AddUnique` (`self.SeenActors`) SeenActor)
    (else
      (`KismetArrayLibrary.Array_RemoveItem` (`self.SeenActors`) SeenActor))))

(fn `SetIsConfused`
  (params (IsConfused :type Boolean))
  (returns (` ` :type Boolean))
  (bind _output_get (set `self.IsConfused` IsConfused))
  (`|ExecutionSequence`
    (:`then_0`
      (if _output_get
        (`self.OnWake`)
        (else
          (`self.OnIdle`))))
    (:`then_1`
      (return _output_get))))

(fn `SetOperator`
  (params (Operator :type "Actor Object Reference"))
  (returns (` ` :type "Actor Object Reference"))
  (bind _output_get (set `self.Operator` Operator))
  (return _output_get))