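; Endless scrolling forest with road traffic, faking forward travel by moving instanced trees and cars instead of the viewer.
; Construction randomly scatters two tree patches on both sides of a central gap and spaces cars along one lane.
; UpdatePosition sets lateral Scene position, shifts instances backward by per-component speed, and recycles those behind MinimumX to MaxDistance, optionally re-randomized.
; Only one instance update per component dirties render state.
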(event `UpdatePosition`
  (params (Offset :type "Float (double-precision)") (YPosition :type "Float (double-precision)"))
  (bind _returnvalue (`KismetMathLibrary.RandomFloatInRange` 1.0 2.0))
  (bind _minwidth (`self.MinWidth`))
  (bind _returnvalue_2 (`KismetMathLibrary.Conv_IntToDouble` (`self.MaxDistance`)))
  (`SceneComponent.K2_SetRelativeLocation` (`self.Scene`) (`KismetMathLibrary.MakeVector` 0.0 YPosition) false false)
  (for (_array_element _array_index) (`|MakeArray` (`self.TreePatch1`) (`self.TreePatch2`) (`self.Car`))
    (bind _returnvalue_3 (- (`InstancedStaticMeshComponent.GetInstanceCount` _array_element) 1))
    (for _index (range (+ _returnvalue_3 1))
      (bind _returnvalue_4 (- _returnvalue_3 _index))
      (bind _x (.x (.location (`InstancedStaticMeshComponent.GetInstanceTransform` _array_element _returnvalue_4 false))))
      (if (< _x (`KismetMathLibrary.Conv_IntToDouble` (`self.MinimumX`)))
        (bind _returnvalue_5 (== _returnvalue_4 _returnvalue_3))
        (`InstancedStaticMeshComponent.UpdateInstanceTransform` _array_element _returnvalue_4 (select `bool` (`|GetArrayItem` (`self.RandomizeY`) _array_index) :`false` (`KismetMathLibrary.MakeTransform` (`KismetMathLibrary.MakeVector` _returnvalue_2 (.y (.location (`InstancedStaticMeshComponent.GetInstanceTransform` _array_element _returnvalue_4 false))) (.z (.location (`InstancedStaticMeshComponent.GetInstanceTransform` _array_element _returnvalue_4 false)))) (.rotation (`InstancedStaticMeshComponent.GetInstanceTransform` _array_element _returnvalue_4 false)) (.scale (`InstancedStaticMeshComponent.GetInstanceTransform` _array_element _returnvalue_4 false))) :`true` (`KismetMathLibrary.MakeTransform` (`KismetMathLibrary.MakeVector` _returnvalue_2 (* (`KismetMathLibrary.RandomFloatInRange` (`KismetMathLibrary.Conv_IntToDouble` _minwidth) (`KismetMathLibrary.Conv_IntToDouble` (+ _minwidth (`self.Width`)))) (select `bool` (`KismetMathLibrary.RandomBool`) :`false` -1.0 :`true` 1.0 :!type "Float (single-precision)"))) (`KismetMathLibrary.MakeRotator` 0.0 0.0 (`KismetMathLibrary.RandomFloatInRange` -180.0 180.0)) (`KismetMathLibrary.MakeVector` _returnvalue _returnvalue _returnvalue))) false _returnvalue_5 false)
        (else
          (`InstancedStaticMeshComponent.UpdateInstanceTransform` _array_element _returnvalue_4 (`KismetMathLibrary.MakeTransform` (`KismetMathLibrary.MakeVector` (+ _x (* (* Offset -1.0) (`|GetArrayItem` (`self.SpeedMultiplier`) _array_index))) (.y (.location (`InstancedStaticMeshComponent.GetInstanceTransform` _array_element _returnvalue_4 false))) (.z (.location (`InstancedStaticMeshComponent.GetInstanceTransform` _array_element _returnvalue_4 false)))) (.rotation (`InstancedStaticMeshComponent.GetInstanceTransform` _array_element _returnvalue_4 false)) (.scale (`InstancedStaticMeshComponent.GetInstanceTransform` _array_element _returnvalue_4 false))) false _returnvalue_5 false))))))

(fn `UserConstructionScript`
  (bind _returnvalue (`KismetMathLibrary.RandomFloatInRange` 1.0 2.0))
  (bind _returnvalue_2 (`KismetMathLibrary.RandomFloatInRange` 1.0 2.0))
  (bind _minwidth (`self.MinWidth`))
  (bind _minwidth_2 (`self.MinWidth`))
  (for _ (range (`self.NumberOfTrees`))
    (`InstancedStaticMeshComponent.AddInstance` (`self.TreePatch1`) (`KismetMathLibrary.MakeTransform` (`KismetMathLibrary.MakeVector` (`KismetMathLibrary.RandomFloatInRange` 100.0 (`KismetMathLibrary.Conv_IntToDouble` (`self.MaxDistance`))) (* (`KismetMathLibrary.RandomFloatInRange` (`KismetMathLibrary.Conv_IntToDouble` _minwidth_2) (`KismetMathLibrary.Conv_IntToDouble` (+ _minwidth_2 (`self.Width`)))) (select `bool` (`KismetMathLibrary.RandomBool`) :`false` -1.0 :`true` 1.0 :!type "Float (single-precision)"))) (`KismetMathLibrary.MakeRotator` 0.0 0.0 (`KismetMathLibrary.RandomFloatInRange` -180.0 180.0)) (`KismetMathLibrary.MakeVector` _returnvalue_2 _returnvalue_2 _returnvalue_2)))
    (`InstancedStaticMeshComponent.AddInstance` (`self.TreePatch2`) (`KismetMathLibrary.MakeTransform` (`KismetMathLibrary.MakeVector` (`KismetMathLibrary.RandomFloatInRange` 100.0 (`KismetMathLibrary.Conv_IntToDouble` (`self.MaxDistance`))) (* (`KismetMathLibrary.RandomFloatInRange` (`KismetMathLibrary.Conv_IntToDouble` _minwidth) (`KismetMathLibrary.Conv_IntToDouble` (+ _minwidth (`self.Width`)))) (select `bool` (`KismetMathLibrary.RandomBool`) :`false` -1.0 :`true` 1.0 :!type "Float (single-precision)"))) (`KismetMathLibrary.MakeRotator` 0.0 0.0 (`KismetMathLibrary.RandomFloatInRange` -180.0 180.0)) (`KismetMathLibrary.MakeVector` _returnvalue _returnvalue _returnvalue))))
  (for _ (range 21)
    (bind _output_get (set `self.Location` (+ (`self.Location`) (`KismetMathLibrary.RandomFloatInRange` 5000.0 (+ (* (`self.MaxDistance`) 0.25) 5000.0)))))
    (if (< _output_get (`KismetMathLibrary.Conv_IntToDouble` (`self.MaxDistance`)))
      (`InstancedStaticMeshComponent.AddInstance` (`self.Car`) (`KismetMathLibrary.MakeTransform` (`KismetMathLibrary.MakeVector` _output_get -260.0) (struct :`Yaw` 180.0))))))