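; First-person player character for a Payday-style heist game, handling movement, hitscan fire, interaction and loot bags.
; Use traces for a target and runs timed interactions with a progress widget; bag type scales walk speed and throw force.
; An InputOverride macro reroutes Use and Fire while viewing through override cameras, to exit or cycle them.
; It creates the HUD widgets and tracks detecting actors until alarm, selecting the one nearest full alert.
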(event `self.ReceiveBeginPlay`
  (`parent.ReceiveBeginPlay`)
  (`|ExecutionSequence`
    (:`then_0`
      (bind _returnvalue (`|CreateWidget` "/Game/Game/UI/LootWidget.LootWidget_C" null self))
      (`UserWidget.AddToViewport` _returnvalue 0))
    (:`then_1`
      (bind _returnvalue_2 (`|CreateWidget` "/Game/Game/UI/ScoreWidget.ScoreWidget_C"))
      (`UserWidget.AddToViewport` _returnvalue_2 0))
    (:`then_2`
      (bind _returnvalue_3 (`|CreateWidget` "/Game/Game/UI/DetectionWidget.DetectionWidget_C" null 0.8))
      (bind _output_get (set `self.DetectionMeterWidget` _returnvalue_3))
      (`UserWidget.AddToViewport` _output_get 0))
    (:`then_3`
      (bind _returnvalue_4 (`|CreateWidget` "/Game/Game/UI/HudWidget.HudWidget_C"))
      (bind _output_get_2 (set `self.HudWidget` _returnvalue_4))
      (`UserWidget.AddToViewport` _output_get_2 0))
    (:`then_4`
      (bind _asheist_game_clone_game_state (cast `/Game/Game/Blueprints/HeistGameCloneGameState` (`GameplayStatics.GetGameState`)))
      (add `/Game/Game/Blueprints/HeistGameCloneGameState.UpdateAlarmState` _asheist_game_clone_game_state (`|CreateDelegate` :!event `SetOffAlarm`)))
    (:`then_5`
      (bind _asplayer_controller (cast `PlayerController` (`self.GetController`)))
      (set `PlayerController.bShowMouseCursor` false _asplayer_controller)
      (`WidgetBlueprintLibrary.SetInputMode_GameOnly` _asplayer_controller))))

(event `InputAction|Crouch`
  (params (Key :type "Key Structure"))
  (:`Pressed`
    (`self.InputOverride` :!label _label
      (:`Pressed `
        (set `self.IsCrouchDown` true)
        (`/Engine/EditorBlueprintResources/StandardMacros.FlipFlop`
          (:`A`
            (`self.Crouch`))
          (:`B`
            (`self.UnCrouch`))))
      (:`Released `
        (set `self.IsCrouchDown` false))))
  (:`Released`
    (goto _label :!via `Released`)))

(event `EndInteractionOnTimer`
  (`self.FinishInteraction` true))

(event `InputAction|Use`
  (params (Key :type "Key Structure"))
  (:`Pressed`
    (`self.InputOverride` :!label _label_2
      (:`Pressed `
        (bind (_success _hitresult _hitactor _hitcomponent) (`self.LookTrace`))
        (if _success
          (bind _caninteract (message `/Game/Game/Blueprints/InteractionInterface.CanInteract` _hitactor))
          (if _caninteract
            (set `self.InteractionTarget` _hitactor)
            (bind _bagtype (message `/Game/Game/Blueprints/LootableInterface.GetBagInfo` (`self.InteractionTarget`)))
            (if (`|EnumEquality` _bagtype "NewEnumerator4")
              (bind _doesblockmovement (message `/Game/Game/Blueprints/InteractionInterface.GetBlocksMovement` (`self.InteractionTarget`) :!label _label_3))
              (`self.SetIgnoreMovementInput` _doesblockmovement)
              (message `/Game/Game/Blueprints/InteractionInterface.BeginInteraction` (`self.InteractionTarget`) (`self.GetController`) self _hitcomponent)
              (bind _duration (message `/Game/Game/Blueprints/InteractionInterface.GetInteractionDuration` (`self.InteractionTarget`)))
              (if (> _duration 0.0)
                (bind _returnvalue (`KismetSystemLibrary.K2_SetTimerDelegate` (delegate `EndInteractionOnTimer`) _duration))
                (bind _output_get (set `self.InteractionTimerHandle` _returnvalue))
                (bind _text (message `/Game/Game/Blueprints/InteractionInterface.GetInteractionText` (`self.InteractionTarget`)))
                (bind _returnvalue_2 (`|CreateWidget` "/Game/Game/UI/InteractionWidget.InteractionWidget_C" (cast `PlayerController` (`self.GetController`) :!pure true) _output_get _text))
                (bind _output_get_2 (set `self.InteractionWidget` _returnvalue_2))
                (`UserWidget.AddToViewport` _output_get_2 0))
              (elif (not (`self.IsCarryingBag`))
                (goto _label_3)
                (else
                  (set `self.InteractionTarget` null)))))))
      (:`Released `
        (`self.FinishInteraction` false))
      (:`OverridePressed`
        (`self.ChangePerspective` null)
        (`KismetArrayLibrary.Array_Clear` (`self.ViewCameraOverrideList`)))))
  (:`Released`
    (goto _label_2 :!via `Released`)))

(event `InputAction|DropBag`
  (params (Key :type "Key Structure"))
  (:`Pressed`
    (`self.InputOverride`
      (:`Pressed `
        (`self.DropBag`)))))

(event `self.ReceiveTick`
  (params (DeltaSeconds :type "Float (single-precision)")))

(event `SetOffAlarm`
  (set `self.IsAlarmState` true)
  (`KismetArrayLibrary.Array_Clear` (`self.Detections`)))

(event `InputAction|Sprint`
  (params (Key :type "Key Structure"))
  (:`Pressed`
    (`self.InputOverride` :!label _label_4
      (:`Pressed `
        (set `self.IsSprinting` true)
        (if (not (`self.IsCrouchDown`))
          (`self.UnCrouch`)))
      (:`Released `
        (set `self.IsSprinting` false)))
    (`self.UpdateWalkSpeed`))
  (:`Released`
    (goto _label_4 :!via `Released`)))

(event `InputAction|Fire`
  (params (Key :type "Key Structure"))
  (bind _firstpersoncamera (`self.FirstPersonCamera`))
  (bind _returnvalue (`SceneComponent.K2_GetComponentLocation` _firstpersoncamera))
  (:`Pressed`
    (`self.InputOverride` :!label _label_5
      (:`Pressed `
        (if true
          (bind (_outhit _returnvalue_2) (`KismetSystemLibrary.LineTraceSingle` :`Start` _returnvalue :`End` (+ _returnvalue (* (`SceneComponent.GetForwardVector` _firstpersoncamera) 10000.0)) :`TraceChannel` "TraceTypeQuery2" :`DrawDebugType` "ForDuration" :`DrawTime` 0.5))
          (if _returnvalue_2
            (bind (_bblockinghit _binitialoverlap _time _distance _location _impactpoint _normal _impactnormal _physmat _hitactor) (`GameplayStatics.BreakHitResult` _outhit))
            (`/Engine/EditorBlueprintResources/StandardMacros.IsValid` _hitactor
              (:`Is Valid`
                (`GameplayStatics.ApplyDamage` _hitactor 10.0 (`self.GetController`) self "/Script/Engine.DamageType"))))))
      (:`OverridePressed`
        (set `self.ViewCameraOverrideIndex` (mod (+ (`self.ViewCameraOverrideIndex`) 1) (`KismetArrayLibrary.Array_Length` (`self.ViewCameraOverrideList`))))
        (`self.ChangePerspective` (`|GetArrayItem` (`self.ViewCameraOverrideList`) (`self.ViewCameraOverrideIndex`)) :!label _label_6))))
  (:`Released`
    (goto _label_5 :!via `Released`)))

(event `InputTouch` :consume false
  (params (Location :type "Vector Structure") (FingerIndex :type "ETouchIndex Enum"))
  (:`Pressed`
    (goto _label_5))
  (:`Released`
    (goto _label_5 :!via `Released`)))

(event `InputAction|SecondaryFire`
  (params (Key :type "Key Structure"))
  (bind _returnvalue (- (`self.ViewCameraOverrideIndex`) 1))
  (:`Pressed`
    (set `self.ViewCameraOverrideIndex` (select `bool` (>= _returnvalue 0) :`false` (- (`KismetArrayLibrary.Array_Length` (`self.ViewCameraOverrideList`)) 1) :`true` _returnvalue))
    (goto _label_6)))

(event `ChangePerspective`
  (params (TargetCamera :type "Actor Object Reference"))
  (bind _viewcamerawidget (`self.ViewCameraWidget`))
  (bind _output_get (set `self.ViewCameraOverride` TargetCamera))
  (`/Engine/EditorBlueprintResources/StandardMacros.IsValid` (`self.ViewCameraWidget`)
    (:`Is Valid`
      (`/Game/Game/UI/ViewCameraWidget.ChangeCamera` (`self.ViewCameraWidget`) _output_get :!label _label_7))
    (:`Is Not Valid`
      (bind _asplayer_controller (cast `PlayerController` (`self.GetController`))
        (:`then`
          (bind _returnvalue (`|CreateWidget` "/Game/Game/UI/ViewCameraWidget.ViewCameraWidget_C" _asplayer_controller _output_get))
          (bind _output_get_2 (set `self.ViewCameraWidget` _returnvalue))
          (`UserWidget.AddToViewport` _output_get_2 0)
          (goto _label_7))
        (:`CastFailed`
          _))))
  (`/Engine/EditorBlueprintResources/StandardMacros.IsValid` _output_get
    (:`Is Valid`
      (bind _asplayer_controller_2 (cast `PlayerController` (`self.GetController`)))
      (`PlayerController.SetViewTargetWithBlend` _asplayer_controller_2 (`self.ViewCameraOverride`) 0.0 "VTBlend_Linear" 0.0 false))
    (:`Is Not Valid`
      (bind _asplayer_controller_3 (cast `PlayerController` (`self.GetController`)))
      (`PlayerController.SetViewTargetWithBlend` _asplayer_controller_3 self 0.0 "VTBlend_Linear" 0.0 false)
      (`self.SetIgnoreMovementInput` false)
      (`/Engine/EditorBlueprintResources/StandardMacros.IsValid` _viewcamerawidget
        (:`Is Valid`
          (`Widget.RemoveFromParent` _viewcamerawidget)
          (set `self.ViewCameraWidget` null))))))

(event `SetCameraOverrideList`
  (params (CameraList :type "Array of Actor Object Reference") (StartIndex :type Integer))
  (set `self.ViewCameraOverrideList` CameraList)
  (bind _output_get (set `self.ViewCameraOverrideIndex` StartIndex))
  (bind _output (`|GetArrayItem` (`self.ViewCameraOverrideList`) _output_get))
  (`/Engine/EditorBlueprintResources/StandardMacros.IsValid` _output
    (:`Is Valid`
      (`self.ChangePerspective` _output)
      (`self.SetIgnoreMovementInput` true))))

(fn `AddBag`
  (params (BagType :type "/Game/Game/Blueprints/EBagType Enum" :default "NewEnumerator0"))
  (returns (Success :type Boolean))
  (if (`self.IsCarryingBag`)
    (return false)
    (else
      (set `self.CurrentBagType` BagType)
      (set `self.IsCarryingBag` true)
      (`self.UpdateWalkSpeed`)
      (`self.UpdateBagGraphics`)
      (return true))))

(fn `DropBag`
  (if (`self.IsCarryingBag`)
    (bind _returnvalue (`|SpawnActorFromClass` "/Game/Game/Props/LootBag.LootBag_C" (`KismetMathLibrary.MakeTransform` (- (`SceneComponent.K2_GetComponentLocation` (`self.ThrowBagLocation`)) (0.0 0.0 20.0)) (`SceneComponent.K2_GetComponentRotation` (`self.FirstPersonCamera`))) "AlwaysSpawn" "OverrideRootScale" null (`self.CurrentBagType`) null))
    (`PrimitiveComponent.AddImpulse` (`/Game/Game/Props/LootBox.StaticMesh` _returnvalue) (* (`SceneComponent.GetForwardVector` (`self.FirstPersonCamera`)) (* (`self.ThrowForce`) (`self.GetThrowForceMultiplier` (`self.CurrentBagType`)))) "None" true)
    (set `self.IsCarryingBag` false)
    (set `self.CurrentBagType` "NewEnumerator4")
    (`self.UpdateWalkSpeed`)
    (`self.UpdateBagGraphics`)))

(fn `FinishInteraction`
  (params (FinishedTimer :type Boolean))
  (bind _interactionwidget (`self.InteractionWidget`))
  (`|ExecutionSequence`
    (:`then_0`
      (bind _doesblockmovement (message `/Game/Game/Blueprints/InteractionInterface.GetBlocksMovement` (`self.InteractionTarget`)))
      (if _doesblockmovement
        (`self.SetIgnoreMovementInput` false)))
    (:`then_1`
      (`KismetSystemLibrary.K2_ClearAndInvalidateTimerHandle` (`self.InteractionTimerHandle`))
      (`/Engine/EditorBlueprintResources/StandardMacros.IsValid` (`self.InteractionTarget`)
        (:`Is Valid`
          (message `/Game/Game/Blueprints/InteractionInterface.EndInteraction` (`self.InteractionTarget`) (`self.GetController`) self FinishedTimer))
        (:`Is Not Valid`
          _))
      (set `self.InteractionTarget` null))
    (:`then_2`
      (`/Engine/EditorBlueprintResources/StandardMacros.IsValid` _interactionwidget
        (:`Is Valid`
          (`Widget.RemoveFromParent` _interactionwidget)
          (set `self.InteractionWidget` null))))))

(fn `GetClosestDetectionAmount`)

(fn `GetDetectionRange`
  (returns (Range :type "Float (double-precision)"))
  (return (select `bool` (`self.bIsCrouched`) :`false` 1.0 :`true` 0.5 :!type "Float (single-precision)")))

(fn `GetIsDetected`
  (returns (ReturnValue :type Boolean))
  (return (> (`KismetArrayLibrary.Array_Length` (`self.Detections`)) 0)))

(fn `GetThrowForceMultiplier`
  (params (BagType :type "/Game/Game/Blueprints/EBagType Enum" :default "NewEnumerator4"))
  (returns (ForceMultiplier :type "Float (double-precision)"))
  (return (select `/Game/Game/Blueprints/EBagType` BagType :`NewEnumerator4` 1.0 :`NewEnumerator0` 0.5 :`NewEnumerator1` 1.2 :`NewEnumerator2` 0.8 :`NewEnumerator3` 1.0 :!type "Float (single-precision)")))

(fn `LookTrace`
  (returns (Success :type Boolean) (HitResult :type "HitResult Structure") (HitActor :type "Actor Object Reference") (HitComponent :type "PrimitiveComponent Object Reference"))
  (bind _firstpersoncamera (`self.FirstPersonCamera`))
  (bind _returnvalue (`SceneComponent.K2_GetComponentLocation` _firstpersoncamera))
  (bind (_outhit _returnvalue_2) (`KismetSystemLibrary.LineTraceSingle` _returnvalue (+ _returnvalue (* (`SceneComponent.GetForwardVector` _firstpersoncamera) (`self.InteractRange`))) "TraceTypeQuery3"))
  (bind (_bblockinghit _binitialoverlap _time _distance _location _impactpoint _normal _impactnormal _physmat _hitactor _hitcomponent) (`GameplayStatics.BreakHitResult` _outhit))
  (return _returnvalue_2 _outhit _hitactor _hitcomponent))

(fn `RegisterDetection`
  (params (SensingActor :type "Actor Object Reference (by ref)"))
  (if (not (`self.IsAlarmState`))
    (`KismetArrayLibrary.Array_AddUnique` (`self.Detections`) SensingActor)
    (`self.UpdateClosestDetector`)))

(fn `SetIgnoreMovementInput`
  (params (bNewMoveInput :type Boolean))
  (returns (ReturnValue :type Boolean))
  (bind _asplayer_controller (cast `PlayerController` (`self.GetController`))
    (:`then`
      (`Controller.SetIgnoreMoveInput` _asplayer_controller bNewMoveInput))
    (:`CastFailed`
      _))
  (if (and (`self.IsMoveInputIgnored`) true)
    (`NavMovementComponent.StopActiveMovement` (`self.CharacterMovement`)))
  (return (`self.IsMoveInputIgnored`)))

(fn `UnregisterDetection`
  (params (SensingActor :type "Actor Object Reference (by ref)"))
  (`|ExecutionSequence`
    (:`then_0`
      (if (!= (`KismetArrayLibrary.Array_Find` (`self.Detections`) SensingActor) -1)
        (`KismetArrayLibrary.Array_RemoveItem` (`self.Detections`) SensingActor)))
    (:`then_1`
      (`self.UpdateClosestDetector`))))

(fn `UpdateBagGraphics`
  (bind _returnvalue (`self.GetController`))
  (`Controller.SetControlRotation` _returnvalue (`KismetMathLibrary.MakeRotator` (select `bool` (`self.IsCarryingBag`) :`true` -5.0 :!type "Float (single-precision)") (.pitch (`Controller.GetControlRotation` _returnvalue)) (.yaw (`Controller.GetControlRotation` _returnvalue)))))

(fn `UpdateClosestDetector`
  (returns (ClosestDetector :type "Actor Object Reference"))
  (locals (LocalCurrentClosest :type "Actor Object Reference") (LocalCurrentClosestTimer :type "Float (double-precision)"))
  (`|ExecutionSequence`
    (:`then_0`
      (if (> (`KismetArrayLibrary.Array_Length` (`self.Detections`)) 0)
        (set `local.LocalCurrentClosestTimer` 5000.0)
        (for _array_element (`self.Detections`)
          (bind _returnvalue (`self.GetComponentByClass` _array_element "/Game/Game/Blueprints/Enemies/Behavior/DetectionHandler.DetectionHandler_C"))
          (`/Engine/EditorBlueprintResources/StandardMacros.IsValid` _returnvalue
            (:`Is Valid`
              (if (`|EnumInequality` (`/Game/Game/Blueprints/Enemies/Behavior/DetectionHandler.GetDetectionState` _returnvalue) "NewEnumerator0")
                (bind _returnvalue_2 (- (`/Game/Game/Blueprints/Enemies/Behavior/DetectionHandler.GetAlertDuration` _returnvalue) (`/Game/Game/Blueprints/Enemies/Behavior/DetectionHandler.GetAlertLevel` _returnvalue)))
                (if (< _returnvalue_2 (`local.LocalCurrentClosestTimer`))
                  (set `local.LocalCurrentClosestTimer` _returnvalue_2)
                  (set `local.LocalCurrentClosest` _array_element))))))
        (if (!= (`local.LocalCurrentClosest`) (`self.ClosestDetector`))
          (bind _output_get (set `self.ClosestDetector` (`local.LocalCurrentClosest`)))
          (`self.UpdateDetectionMeter`)
          (return _output_get)
          (else
            (return (`self.ClosestDetector`))))))
    (:`then_1`
      (bind _output_get_2 (set `self.ClosestDetector` null))
      (`self.UpdateDetectionMeter`)
      (return _output_get_2))))

(fn `UpdateWalkSpeed`
  (bind _charactermovement (`self.CharacterMovement`))
  (bind _output_get (set `CharacterMovementComponent.MaxWalkSpeed` (select `bool` (`self.IsSprinting`) :`false` (* 400.0 (select `bool` (`self.IsCarryingBag`) :`false` 1.0 :`true` (`KismetMathLibrary.FClamp` (`self.GetThrowForceMultiplier` (`self.CurrentBagType`)) 0.5))) :`true` (* 800.0 (select `bool` (`self.IsCarryingBag`) :`false` 1.0 :`true` (`KismetMathLibrary.FClamp` (`self.GetThrowForceMultiplier` (`self.CurrentBagType`)) 0.5)))) _charactermovement))
  (set `CharacterMovementComponent.MaxWalkSpeedCrouched` (* _output_get 0.5) _charactermovement))

(fn `UserConstructionScript`
  (`parent.UserConstructionScript`))