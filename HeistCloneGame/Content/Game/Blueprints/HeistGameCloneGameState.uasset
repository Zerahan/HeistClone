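; Heist game state that tracks stashed bags, score, exiting players, kills and the alarm countdown.
; BeginPlay randomizes prize values per bag type; reaching the required bag count activates the exit zones.
; With all players in an active exit, TriggerEndGame marks a win, banks carried bags and starts a timer.
; An expired alarm or LoadLevel call returns to the lobby, saving results to the GameInstance; excess guard kills start another delayed event.
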(event `self.ReceiveBeginPlay`
  (set `self.Bags` (`|MakeArray`))
  (`KismetArrayLibrary.Array_Resize` (`self.ExitingPlayers`) (`KismetArrayLibrary.Array_Length` (`self.PlayerArray`)))
  (bind _enumvalue (foreach `/Game/Game/Blueprints/EBagType` false)
    (:`LoopBody`
      (`KismetArrayLibrary.Array_Set` (`self.PrizeValues`) (`KismetMathLibrary.Conv_ByteToInt` _enumvalue) (`KismetMathLibrary.FTrunc` (* (select `/Game/Game/Blueprints/EBagType` _enumvalue :`NewEnumerator1` 20000 :`NewEnumerator2` 100000 :`NewEnumerator3` 50000) (`KismetMathLibrary.RandomFloatInRange` 0.8 1.2))) true))))

(event `TriggerEndGame`
  (if (`self.IsEscapeActive`)
    (if (`KismetSystemLibrary.K2_IsTimerActiveHandle` (`self.EndgameTimerHandle`))
      _
      (elif (`self.AreAllPlayersInExit`)
        (set `self.IsWin` true)
        (bind _returnvalue (`KismetSystemLibrary.K2_SetTimerDelegate` (`|CreateDelegate` :!event `LoadLevel`) 2.0))
        (set `self.EndgameTimerHandle` _returnvalue)
        (set `self.IsEndgameTriggered` true)
        (bind _outactors (`GameplayStatics.GetAllActorsOfClass` "/Game/Game/Blueprints/HeistGameCloneCharacter.HeistGameCloneCharacter_C"))
        (for _array_element _outactors
          (if (`/Game/Game/Blueprints/HeistGameCloneCharacter.IsCarryingBag` _array_element)
            (`self.AddBagToScore` (`/Game/Game/Blueprints/HeistGameCloneCharacter.CurrentBagType` _array_element))))))))

(event `LoadLevel`
  (bind _asheist_game_clone_game_instance (cast `/Game/Game/Blueprints/HeistGameCloneGameInstance` (`GameplayStatics.GetGameInstance`))
    (:`then`
      (`/Game/Game/Blueprints/HeistGameCloneGameInstance.SetLastGameResults` _asheist_game_clone_game_instance (make `/Game/Game/Blueprints/GameResults` (`self.IsWin`) (`self.GetNumberOfBags`) (`self.GetStashedScore`) (`KismetMathLibrary.FFloor` (`KismetSystemLibrary.GetGameTimeInSeconds`)) (`self.KilledGuards`) (`self.KilledCivilians`))))
    (:`CastFailed`
      _))
  (`GameplayStatics.OpenLevel` "dev_Lobby"))

(event `SetOffAlarm`
  (if (not (`self.IsAlarmGoing`))
    (set `self.IsAlarmGoing` true)
    (set `self.GameOverTime` (+ (`KismetSystemLibrary.GetGameTimeInSeconds`) (`self.GameOverTimerLength`)))
    (`self.UpdateAlarmState`)))

(event `self.ReceiveTick`
  (params (DeltaSeconds :type "Float (single-precision)"))
  (if (`self.IsEndgameTriggered`)
    _
    (elif (`self.IsAlarmGoing`)
      (if (< (- (`self.GameOverTime`) (`KismetSystemLibrary.GetGameTimeInSeconds`)) 0.0)
        (`self.LoadLevel`)))))

(event `RegisterGuardDeath`
  (set `self.KilledGuards` (+ (`self.KilledGuards`) 1))
  (if (> (`self.KilledGuards`) (`self.KilledGuardAlarmAmount`))
    (if (not (`self.KilledGuardAlarm`))
      (set `self.KilledGuardAlarm` true)
      (`KismetSystemLibrary.K2_SetTimerDelegate` (`|CreateDelegate` :!event `SetOffAlarm`) 2.0))))

(event `RegisterCivilianDeath`
  (set `self.KilledCivilians` (+ (`self.KilledCivilians`) 1)))

(fn `AddBagToScore`
  (params (BagToAdd :type "/Game/Game/Blueprints/EBagType Enum" :default "NewEnumerator4"))
  (returns (Success :type Boolean))
  (locals (LocalScore :type Integer))
  (if (`self.IsScorableBag` BagToAdd)
    (`KismetArrayLibrary.Array_Add` (`self.Bags`) BagToAdd)
    (for _array_element (`self.Bags`)
      (set `local.LocalScore` (+ (`local.LocalScore`) (`|GetArrayItem` (`self.PrizeValues`) (`KismetMathLibrary.Conv_ByteToInt` _array_element)))))
    (set `self.CurrentScore` (`local.LocalScore`))
    (`self.UpdateScoreInfo`)
    (`|ExecutionSequence`
      (:`then_0`
        (if (not (`self.IsEscapeActive`))
          (if (>= (`self.GetNumberOfBags`) (`self.GetNumBagsForExitZone`))
            (set `self.IsEscapeActive` true)
            (bind _outactors (`GameplayStatics.GetAllActorsOfClass` "/Game/Game/Props/Zone_LevelExit.Zone_LevelExit_C"))
            (for _array_element_2 _outactors
              (`/Game/Game/Props/Zone_LevelExit.SetIsEscapeActive` _array_element_2 true)))))
      (:`then_1`
        (return true)))
    (else
      (return false))))

(fn `AreAllPlayersInExit`
  (returns (AreAllPlayersAtExit :type Boolean))
  (locals (LocalAreAllPlayersAtExit :type Boolean))
  (set `local.LocalAreAllPlayersAtExit` true)
  (for _array_element (`self.ExitingPlayers`)
    (if (not (`KismetSystemLibrary.IsValid` _array_element))
      (set `local.LocalAreAllPlayersAtExit` false)))
  (`KismetSystemLibrary.PrintText` (`|FormatText` "Exit? {AllExit} \nPlayers: {Num}" (`KismetTextLibrary.Conv_BoolToText` (`local.LocalAreAllPlayersAtExit`)) (`KismetArrayLibrary.Array_Length` (`self.ExitingPlayers`))))
  (return (`local.LocalAreAllPlayersAtExit`)))

(fn `GetKilledGuardCount`
  (returns (KilledGuards :type Integer) (KilledGuardAlarmAmount :type Integer))
  (return (`self.KilledGuards`) (`self.KilledGuardAlarmAmount`)))

(fn `GetNumBagsForExitZone`
  (returns (RequiredBagCount :type Integer))
  (return (`self.RequiredBagCount`)))

(fn `GetNumberOfBags`
  (returns (ReturnValue :type Integer))
  (return (`KismetArrayLibrary.Array_Length` (`self.Bags`))))

(fn `GetStashedScore`
  (returns (CurrentScore :type Integer))
  (return (`self.CurrentScore`)))

(fn `GetTimer`
  (returns (ReturnValue :type "Float (double-precision)"))
  (return (select `bool` (`self.IsAlarmGoing`) :`false` (`KismetSystemLibrary.GetGameTimeInSeconds`) :`true` (- (`self.GameOverTime`) (`KismetSystemLibrary.GetGameTimeInSeconds`)))))

(fn `IsScorableBag`
  (params (BagToScore :type "/Game/Game/Blueprints/EBagType Enum" :default "NewEnumerator4"))
  (returns (ReturnValue :type Boolean))
  (return (and (`|EnumInequality` BagToScore "NewEnumerator4") (`|EnumInequality` BagToScore "NewEnumerator0"))))

(fn `RegisterPlayerAtExit`
  (params (Character :type "/Game/Game/Blueprints/HeistGameCloneCharacter Object Reference"))
  (bind _asplayer_controller (cast `PlayerController` (`Pawn.GetController` Character)))
  (`KismetArrayLibrary.Array_Set` (`self.ExitingPlayers`) (`GameplayStatics.GetPlayerControllerID` _asplayer_controller) Character)
  (return))

(fn `UnregisterPlayerAtExit`
  (params (Character :type "/Game/Game/Blueprints/HeistGameCloneCharacter Object Reference (by ref)"))
  (bind _asplayer_controller (cast `PlayerController` (`Pawn.GetController` Character)))
  (`KismetArrayLibrary.Array_Set` (`self.ExitingPlayers`) (`GameplayStatics.GetPlayerControllerID` _asplayer_controller)))

(fn `UserConstructionScript`)