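; LobbyPawn is the lobby's pawn, showing the lobby menu over a camera view that follows the mouse.
; On BeginPlay it creates LobbyMenuWidget, adds it to the viewport, then switches the player controller to UI-only input with a visible cursor.
; Each tick it maps the cursor's viewport-relative position to camera pitch and yaw, scaled by RotationRange, with yaw weighted more strongly.
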(event `self.ReceiveBeginPlay`
  (bind _returnvalue (`|CreateWidget` "/Game/Game/UI/LobbyMenuWidget.LobbyMenuWidget_C"))
  (bind _output_get (set `self.MenuWidget` _returnvalue))
  (`UserWidget.AddToViewport` _output_get 0)
  (bind _asplayer_controller (cast `PlayerController` (`self.GetController`)))
  (`WidgetBlueprintLibrary.SetInputMode_UIOnlyEx` _asplayer_controller (`self.MenuWidget`))
  (set `PlayerController.bShowMouseCursor` true _asplayer_controller))

(event `self.ReceiveTick`
  (params (DeltaSeconds :type "Float (single-precision)"))
  (bind _rotationrange (`self.RotationRange`))
  (bind _returnvalue (`WidgetLayoutLibrary.GetMousePositionOnViewport`))
  (bind (_x _y) (`KismetMathLibrary.BreakVector2D` (* (/ _returnvalue (`WidgetLayoutLibrary.GetViewportSize`)) 2.5)))
  (`SceneComponent.K2_SetRelativeRotation` (`self.Camera`) (`KismetMathLibrary.MakeRotator` 0.0 (* (- _y 1.0) _rotationrange -1.0) (* (- _x 1.0) _rotationrange 2.0)) false false))

(fn `UserConstructionScript`)