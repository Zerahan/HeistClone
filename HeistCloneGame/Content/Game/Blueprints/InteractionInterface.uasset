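; Blueprint interface that interactable objects implement so a player controller and pawn can interact with them.
; Begin and end calls carry the instigator, with the hit component on begin and a finished-timer value on end, pointing to timed interactions.
; Query functions report whether interaction is allowed, its duration, movement blocking, camera look limits, and the prompt icon and text.
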(fn `BeginInteraction`
  (params (InstigatingController :type "Controller Object Reference") (InstigatingPawn :type "Pawn Object Reference") (HitComponent :type "PrimitiveComponent Object Reference")))

(fn `CanInteract`
  (returns (CanInteract :type Boolean))
  (return false))

(fn `EndInteraction`
  (params (InstigatingController :type "Controller Object Reference") (InstigatingPawn :type "Pawn Object Reference") (FinishedTimer :type Boolean)))

(fn `GetBlocksMovement`
  (returns (DoesBlockMovement :type Boolean))
  (return false))

(fn `GetInteractionDuration`
  (returns (Duration :type "Float (double-precision)"))
  (return 0.0))

(fn `GetInteractionIcon`
  (returns (Icon :type "Texture2D Object Reference"))
  (return null))

(fn `GetInteractionText`
  (returns (Text :type Text))
  (return ""))

(fn `GetLookLimit`
  (returns (HasLimit :type Boolean) (MaxPitchOffset :type "Float (double-precision)") (MaxYawOffset :type "Float (double-precision)"))
  (return false 0.0 0.0))